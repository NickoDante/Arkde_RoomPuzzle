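; BP_Character is a player character Blueprint with an ultimate ability and a choice of first- or third-person view.
; The construction script sets auto-activation on either the FPS camera or the TPS camera and spring arm from UseFirstPersonView.
; BeginPlay adds the BP_Sight widget to the viewport.
; Ultimate events only print colored debug messages for XP gain, start, stop and duration; none of them changes ultimate state here.
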(event EventBeginPlay
  (bind _returnvalue (UserInterface|CreateWidget "/Game/Widgets/BP_Sight.BP_Sight_C"))
  (UserInterface|Viewport|AddtoViewport _returnvalue 0))

(event EventStartUltimate
  (Development|PrintString "Starting Ultimate !!!" true true "(R=1.000000,G=0.208814,B=0.000000,A=1.000000)" 1e+01))

(event EventStopUltimate
  (Development|PrintString "Stopping Ultimate !!!" true true "(R=1.000000,G=0.000000,B=0.091064,A=1.000000)" 1e+01))

(event EventGainUltimateXP
  (params (XPGained :type Float%20%28single-precision%29))
  (Development|PrintString (Utilities|String|Append "XPGained: " (Utilities|String|ToString(Float) XPGained) " || UltimateXP:  " (Utilities|String|ToString(Float) (Variables|Default|GetCurrentUltimateXP)) "/" (Utilities|String|ToString(Float) (Variables|Default|GetMaxUltimateXP))) true true (select (Variables|Default|GetbCanUseUltimate) "(R=0.000000,G=1.000000,B=0.276276,A=1.000000)" "(R=0.072917,G=0.704225,B=1.000000,A=1.000000)") 5.0))

(event EventUpdateUltimateDuration
  (params (Value :type Float%20%28single-precision%29))
  (Development|PrintString (Utilities|String|Append (Utilities|String|ToString(Float) (Variables|Default|GetCurrentUltimateDuration)) "/" (Utilities|String|ToString(Float) (Variables|Default|GetMaxUltimateDuration))) true true "(R=0.000000,G=0.660000,B=1.000000,A=1.000000)" 5.0))

(fn ConstructionScript
  (Components|Activation|SetAutoActivate (Variables|Default|GetFPSCameraComponent) (Variables|Default|GetbUseFirstPersonView))
  (Components|Activation|SetAutoActivate (Variables|Default|GetTPSCameraComponent) (not (Variables|Default|GetbUseFirstPersonView))))